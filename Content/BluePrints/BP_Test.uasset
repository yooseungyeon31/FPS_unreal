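; BP_Test is a test actor that oscillates back and forth along a straight line.
; Each Tick accumulates running time and feeds it, scaled by MoveSpeed, into a sine wave with MoveDistance as amplitude.
; The offset from StartLocation follows the right vector of a zero rotation, so motion is on world Y, applied without sweep.
; The graphs shown never assign StartLocation.
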(event EventTick
  (params (DeltaSeconds :type Float%20%28single-precision%29))
  (bind _output_get (Variables|Default|SetRunning%20Time (+ DeltaSeconds (Variables|Default|GetRunning%20Time))))
  (Transformation|SetActorLocation (+ (Variables|Default|GetStartLocation) (* (* (Math|Trig|Sin(Radians) (* _output_get (Variables|Default|GetMoveSpeed))) (Variables|Default|GetMoveDistance)) (Math|Vector|GetRightVector "0, 0, 0"))) false false))

(fn ConstructionScript)